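; A spline actor that builds a chain of mesh segments along its editable path.
; Its construction script adds one spline mesh component per pair of neighboring spline points and attaches it to the Scene component.
; Each segment takes its start and end from the local locations and tangents of those points, so the chain follows the curve.
; The event graph has no runtime logic.
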(event `self.ReceiveBeginPlay`)

(event `self.ReceiveActorBeginOverlap`
  (params (OtherActor :type "Actor Object Reference")))

(event `self.ReceiveTick`
  (params (DeltaSeconds :type "Float (single-precision)")))

(fn `UserConstructionScript`
  (bind _spline (`self.Spline`))
  (for _index (range (+ (- (`SplineComponent.GetNumSplinePoints`) 2) 1))
    (bind _returnvalue (`AddComponent|Spline Mesh Component_1` :`bManualAttachment` true))
    (`SceneComponent.K2_AttachTo` _returnvalue (`self.Scene`) "None" "KeepRelativeOffset" true)
    (bind (_locallocation _localtangent) (`SplineComponent.GetLocalLocationAndTangentAtSplinePoint` _spline _index))
    (bind (_locallocation_2 _localtangent_2) (`SplineComponent.GetLocalLocationAndTangentAtSplinePoint` _spline (+ _index 1)))
    (`SplineMeshComponent.SetStartAndEnd` _returnvalue _locallocation _localtangent _locallocation_2 _localtangent_2)))