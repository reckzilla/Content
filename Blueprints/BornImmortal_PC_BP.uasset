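; Player controller for BornImmortal that manages the HUD, inventory menu and pause menu.
; On BeginPlay it caches the player character and adds the HUD widget to the viewport.
; The InventoryMenu and Pause inputs each toggle game pause, swap the HUD for a freshly created menu widget and show the mouse cursor.
; IsInventory and IsPaused flags keep the two menus mutually exclusive.
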(event `self.ReceiveBeginPlay`
  (bind _asborn_immortal_character (cast `BornImmortalCharacter` (`GameplayStatics.GetPlayerCharacter` null)))
  (set `self.BIPlayer` _asborn_immortal_character)
  (bind _returnvalue (`|CreateWidget` "/Game/Blueprints/UI/HUD/HUD_UI.HUD_UI_C" self))
  (set `self.UI` _returnvalue)
  (`UserWidget.AddToViewport` _returnvalue 0))

(event `InputAction|InventoryMenu` :paused true
  (bind _ui (`self.UI`))
  (:`Pressed`
    (if (`self.IsPaused`)
      _
      (elif (`self.IsInventory`)
        (set `self.IsInventory` false)
        (`GameplayStatics.SetGamePaused` (`self.BIPlayer`))
        (`UserWidget.AddToViewport` _ui 0)
        (`Widget.RemoveFromParent` (`self.InventoryUI`))
        (set `PlayerController.bShowMouseCursor` false)
        (else
          (set `self.IsInventory` true)
          (`GameplayStatics.SetGamePaused` (`self.BIPlayer`) true)
          (`Widget.RemoveFromParent` _ui)
          (bind _returnvalue (`|CreateWidget` "/Game/Blueprints/UI/Inventory/Inventory_Menu_Prototype.Inventory_Menu_Prototype_C" self))
          (bind _output_get (set `self.InventoryUI` _returnvalue))
          (`UserWidget.AddToViewport` _output_get 0)
          (set `PlayerController.bShowMouseCursor` true))))))

(event `InputAction|Pause` :paused true
  (bind _ui (`self.UI`))
  (:`Pressed`
    (if (`self.IsInventory`)
      _
      (elif (`self.IsPaused`)
        (set `self.IsPaused` false)
        (`GameplayStatics.SetGamePaused` false)
        (`UserWidget.AddToViewport` _ui 0)
        (`Widget.RemoveFromParent` (`self.StartMenu`))
        (set `PlayerController.bShowMouseCursor` false)
        (else
          (set `self.IsPaused` true)
          (`GameplayStatics.SetGamePaused` true)
          (`Widget.RemoveFromParent` _ui)
          (bind _returnvalue (`|CreateWidget` "/Game/Blueprints/UI/StartMenu/StartMenu.StartMenu_C" self))
          (bind _output_get (set `self.StartMenu` _returnvalue))
          (`UserWidget.AddToViewport` _output_get 0)
          (set `PlayerController.bShowMouseCursor` true))))))

(fn `UserConstructionScript`)