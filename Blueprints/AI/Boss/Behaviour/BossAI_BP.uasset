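; AI controller for the boss that starts the Boss_BT behavior tree when it possesses a Boss_BP pawn.
; A looping MultiGate on Tick alternates between two tasks on successive frames.
; One copies the boss's Health into the BossHealth blackboard key.
; The other checks the blackboard State and, on what appears to be the death state, plays the death sound on the mesh and unpossesses the pawn.
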(event `self.ReceiveBeginPlay`)

(event `self.ReceiveTick`
  (params (DeltaSeconds :type "Float (single-precision)"))
  (`|MultiGate` false true 0
    (:`Out 0`
      (bind _asboss_bp (cast `/Game/Blueprints/AI/Boss/Boss_BP` (`self.K2_GetPawn`)))
      (`BlackboardComponent.SetValueAsInt` (`AIBlueprintHelperLibrary.GetBlackboard` null) "BossHealth" (`Enemy.Health` _asboss_bp)))
    (:`Out 1`
      (if (== (`BlackboardComponent.GetValueAsEnum` (`AIBlueprintHelperLibrary.GetBlackboard` null) "State") (enumliteral `/Game/Blueprints/AI/Boss/Behaviour/Boss_State` "NewEnumerator5"))
        (bind _asboss_bp_2 (cast `/Game/Blueprints/AI/Boss/Boss_BP` (`self.K2_GetPawn`)))
        (bind _mesh (`Character.Mesh` _asboss_bp_2))
        (`GameplayStatics.PlaySoundAttached` "/Game/Character/Sounds/Boss/Boss_Death.Boss_Death" _mesh "None" (`SceneComponent.K2_GetComponentLocation` _mesh))
        (`self.UnPossess`)))))

(event `self.OnPossess`
  (params (PossessedPawn :type "Pawn Object Reference"))
  (cast `/Game/Blueprints/AI/Boss/Boss_BP` PossessedPawn)
  (`self.RunBehaviorTree` "/Game/Blueprints/AI/Boss/Behaviour/Boss_BT.Boss_BT"))

(fn `UserConstructionScript`)