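; EnemyAI_BP is the AI controller for the grunt EnemyTest enemy.
; On possession it runs the Enemy_BT behavior tree and seeds the blackboard with a starting Route index and the pawn's IsDead flag.
; Each Tick it checks the controlled pawn and unpossesses it once it is dead.
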(event `self.ReceiveTick`
  (params (DeltaSeconds :type "Float (single-precision)"))
  (bind _asenemy_test (cast `/Game/Blueprints/AI/Grunt/EnemyTest` (`self.K2_GetPawn`)))
  (if (`Enemy.bIsDead` _asenemy_test)
    (`self.UnPossess`)))

(event `self.OnPossess`
  (params (PossessedPawn :type "Pawn Object Reference"))
  (bind _returnvalue (`AIBlueprintHelperLibrary.GetBlackboard` PossessedPawn))
  ;[1 1 1] Initialize Bot AI
  (bind _asenemy_test (cast `/Game/Blueprints/AI/Grunt/EnemyTest` PossessedPawn))
  (`self.RunBehaviorTree` "/Game/Blueprints/AI/Grunt/Behavior/Enemy_BT.Enemy_BT")
  (`BlackboardComponent.SetValueAsInt` _returnvalue "Route" 0)
  (`BlackboardComponent.SetValueAsBool` _returnvalue "IsDead" (`Enemy.bIsDead` _asenemy_test)))

(fn `UserConstructionScript`)